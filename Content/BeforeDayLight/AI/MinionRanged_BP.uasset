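; Ranged minion enemy Blueprint that reacts to damage and to seeing the player, with no attack logic in this graph.
; Health changes from its attribute component spawn a floating damage-number widget while it is alive, or switch the mesh to a custom collision object channel once health runs out.
; Pawn sensing only prints an on-screen "spotted" message when it sees a BDLCharacter.
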(event OnHealthChanged(AttributeComp)
  (params (InstigatorActor :type Actor%20Object%20Reference) (OwningComp :type BDL%20Attribute%20Component%20Object%20Reference) (NewValue :type Float%20%28single-precision%29) (Delta :type Float%20%28single-precision%29))
  (if (> (Class|BDLAttributeComponent|GetCurHealth (Variables|Default|GetAttributeComp)) 0.0)
    (bind _returnvalue (UserInterface|CreateWidget "/Game/BeforeDayLight/UI/DamagePopup_Widget.DamagePopup_Widget_C" 0 self (Math|Float|Truncate Delta)))
    (UserInterface|Viewport|AddtoViewport _returnvalue 0)
    (else
      (Collision|SetCollisionObjectType (Variables|Character|GetMesh) "ECC_GameTraceChannel1"))))

(event OnSeePawn(PawnSensingComp)
  (params (Pawn :type Pawn%20Object%20Reference))
  (Utilities|Casting|CastToBDLCharacter Pawn)
  (Development|PrintString "You are Spotted!!!" true true "(R=1.000000,G=0.087707,B=0.000000,A=1.000000)"))

(event EventBeginPlay)

(event Collision|EventActorBeginOverlap
  (params (OtherActor :type Actor%20Object%20Reference)))

(event EventTick
  (params (DeltaSeconds :type Float%20%28single-precision%29)))

(fn ConstructionScript)